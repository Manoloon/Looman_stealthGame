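; Prototype movement actor that eases itself toward two referenced targets, Target1 and Target2, on Tick.
; Each pass runs through a DoOnce, applying a VInterpTo step toward Target1, then one toward Target2 in the same frame if that move succeeds.
; DoOnce resets only after both non-swept moves succeed, so the actor blends between both pulls rather than visiting each target in turn.
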(event `self.ReceiveTick`
  (params (DeltaSeconds :type "Float (single-precision)"))
  (`/Engine/EditorBlueprintResources/StandardMacros.DoOnce` false :!label _label
    (:`Completed`
      (bind (_sweephitresult _returnvalue) (`self.K2_SetActorLocation` (`KismetMathLibrary.VInterpTo` (`self.K2_GetActorLocation`) (`self.K2_GetActorLocation` (`self.Target1`)) DeltaSeconds 2.0)))
      (if _returnvalue
        (bind (_sweephitresult_2 _returnvalue_2) (`self.K2_SetActorLocation` (`KismetMathLibrary.VInterpTo` (`self.K2_GetActorLocation`) (`self.K2_GetActorLocation` (`self.Target2`)) DeltaSeconds 2.0)))
        (if _returnvalue_2
          (goto _label :!via `Reset`))))))

(fn `UserConstructionScript`)