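; BP_protoBlackHole is a prototype black hole actor that pulls in and destroys static mesh actors.
; Each tick it applies a negative, constant-falloff radial impulse from its location to every StaticMeshActor overlapping its Sphere component, using the sphere's radius as the range.
; Any StaticMeshActor that begins overlapping the central StaticMesh component is destroyed.
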(event `self.ReceiveTick`
  (params (DeltaSeconds :type "Float (single-precision)"))
  (for _array_element (`PrimitiveComponent.GetOverlappingActors` (`self.Sphere`) "/Script/Engine.StaticMeshActor")
    (bind _asstatic_mesh_actor (cast `StaticMeshActor` _array_element))
    (`PrimitiveComponent.AddRadialImpulse` (`StaticMeshActor.StaticMeshComponent` _asstatic_mesh_actor) (`self.K2_GetActorLocation`) (`SphereComponent.SphereRadius` (`self.Sphere`)) -7000.0 "RIF_Constant" false)))

(event `self.StaticMesh.OnComponentBeginOverlap`
  (params (OverlappedComponent :type "PrimitiveComponent Object Reference") (OtherActor :type "Actor Object Reference") (OtherComp :type "PrimitiveComponent Object Reference") (OtherBodyIndex :type Integer) (bFromSweep :type Boolean) (SweepResult :type "HitResult Structure (by ref)"))
  (bind _asstatic_mesh_actor (cast `StaticMeshActor` OtherActor))
  (`self.K2_DestroyActor` _asstatic_mesh_actor))

(fn `UserConstructionScript`)